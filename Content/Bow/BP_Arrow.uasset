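; Bow arrow projectile that flies when fired, sticks into what it hits and reports the impact.
; Fire adds a projectile movement component at runtime, scaling speed and gravity by Strength, then starts trail, sound, collision and lifespan.
; Overlap with non-instigators stops movement, attaches to the closest skeletal bone or hit component, and calls OnArrowImpact.
; Physics-simulating targets receive the launch velocity as an impulse, and only then is the trail destroyed.
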(event `self.ReceiveBeginPlay`
  (`PrimitiveComponent.SetCollisionEnabled` (`self.Box`) "NoCollision"))

(event `Fire`
  (params (Direction :type "Vector Structure") (Strength :type "Float (double-precision)"))
  (set `self.Strength` Strength)
  (bind _returnvalue (`AddComponent|NODE_AddProjectileMovementComponent-0`))
  (set `self.PorjectileMovementComponent` _returnvalue)
  (bind _output_get (set `MovementComponent.Velocity` (* Direction (`KismetMathLibrary.Lerp` (`self.MinSpeed`) (`self.MaxSpeed`) Strength)) _returnvalue))
  (set `self.Velocity` _output_get)
  (set `ProjectileMovementComponent.ProjectileGravityScale` (`KismetMathLibrary.Lerp` (`self.MaxGravity`) (`self.MinGravity`) Strength) _returnvalue)
  (`GameplayStatics.PlaySoundAtLocation` "/Game/Audio/Cue_Arrow_Whoosh.Cue_Arrow_Whoosh" (`self.K2_GetActorLocation`) (struct) 1.0 1.0 0.0 null null null null)
  (bind _returnvalue_2 (`NiagaraFunctionLibrary.SpawnSystemAttached` "/Game/VFX/NS_ArrowTrail.NS_ArrowTrail" (`self.Scene`) "None" (0.0 0.0 0.0) (struct) "KeepRelativeOffset"))
  (set `self.TrailRef` _returnvalue_2)
  (`PrimitiveComponent.SetCollisionEnabled` (`self.Box`) "QueryAndPhysics")
  (`self.SetLifeSpan` 10.0))

(event `self.Box.OnComponentBeginOverlap`
  (params (OverlappedComponent :type "PrimitiveComponent Object Reference") (OtherActor :type "Actor Object Reference") (OtherComp :type "PrimitiveComponent Object Reference") (OtherBodyIndex :type Integer) (bFromSweep :type Boolean) (SweepResult :type "HitResult Structure (by ref)"))
  (bind (_bblockinghit _binitialoverlap _time _distance _location _impactpoint _normal _impactnormal _physmat _hitactor _hitcomponent) (`GameplayStatics.BreakHitResult` SweepResult))
  (bind _returnvalue (`self.GetComponentByClass` _hitactor "/Script/Engine.SkeletalMeshComponent"))
  (if (not (== OtherActor (`self.GetInstigator`)))
    (bind _porjectilemovementcomponent (`self.PorjectileMovementComponent`)
      (:`then`
        (`ActorComponent.K2_DestroyComponent` _porjectilemovementcomponent))
      (:`else`
        _))
    (`PrimitiveComponent.SetCollisionEnabled` (`self.Box`) "NoCollision")
    (`/Engine/EditorBlueprintResources/StandardMacros.IsValid` _returnvalue
      (:`Is Valid`
        (`self.K2_AttachToComponent` _returnvalue (`.ReturnValue` (`SkinnedMeshComponent.FindClosestBone_K2` _returnvalue _location 0.0 false)) "SnapToTarget" "KeepWorld" "KeepWorld"))
      (:`Is Not Valid`
        (`self.K2_AttachToComponent` _hitcomponent "None" "KeepWorld" "KeepRelative" "KeepRelative")))
    (`GameplayStatics.PlaySoundAtLocation` "/Game/Audio/arrow-impact-world.arrow-impact-world" (`self.K2_GetActorLocation`) (struct) 1.0 1.0 0.0 null null null null)
    (`self.OnArrowImpact` (`self.Strength`) _hitactor SweepResult)
    (if (`SceneComponent.IsSimulatingPhysics` _hitcomponent "None")
      (`PrimitiveComponent.AddImpulse` _hitcomponent (`self.Velocity`) "None" true)
      (bind _trailref (`self.TrailRef`)
        (:`then`
          (`ActorComponent.K2_DestroyComponent` _trailref))
        (:`else`)))))

(fn `UserConstructionScript`)