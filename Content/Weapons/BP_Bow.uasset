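; Bow weapon Blueprint that tracks its draw state and plays a draw sound.
; DrawBegin sets the bow state enum, spawns the draw sound at the actor's location and keeps a reference to it.
; DrawEnd switches the state to another value and stops that sound if the reference is still valid.
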(event `DrawBegin`
  (set `self.BowState` "NewEnumerator2")
  (bind _returnvalue (`GameplayStatics.SpawnSoundAtLocation` (`self.DrawSound`) (`self.K2_GetActorLocation`) (struct) 1.0 1.0 0.0 null null))
  (set `self.DrawSoundRef` _returnvalue))

(event `DrawEnd`
  (set `self.BowState` "NewEnumerator0")
  (bind _drawsoundref (`self.DrawSoundRef`)
    (:`then`
      (`AudioComponent.Stop` _drawsoundref))
    (:`else`)))

(fn `UserConstructionScript`
  (`parent.UserConstructionScript`))