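; Bow-wielding enemy AI character that attacks targets at range, built on a parent enemy Blueprint.
; It equips a bow at BeginPlay, and each attack draws, waits a short random delay, fires toward the target's current position, then ends the attack.
; The bow mechanics component reports arrow impacts, which become blockable, non-parryable damage scaled by strength.
; Overrides supply movement speeds per state and equal ideal attack and defend ranges.
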(event `self.ReceiveBeginPlay`
  (`parent.ReceiveBeginPlay`)
  (`/Game/Bow/BPC_Bowmechanics.EquipBow` (`self.BPC_Bowmechanics`)))

(event `self.Attack`
  (params (`Attack Target` :type "Actor Object Reference"))
  (`parent.Attack` `Attack Target`)
  (`/Game/Bow/BPC_Bowmechanics.DrawBegin` (`self.BPC_Bowmechanics`))
  (`KismetSystemLibrary.Delay` (`KismetMathLibrary.RandomFloatInRange` 0.5 1.0))
  (`/Game/Bow/BPC_Bowmechanics.Fire Arrow Begin` (`self.BPC_Bowmechanics`) (`KismetMathLibrary.GetDirectionUnitVector` (`self.K2_GetActorLocation`) (`self.K2_GetActorLocation` `Attack Target`)))
  (`/Game/New_AI/AI/BPI_EnemyAI.AttackEnd` `Attack Target`))

(event `self.BPC_Bowmechanics.OnArrowImpact`
  (params (Strength :type "Float (double-precision)") (`Hit Actor` :type "Actor Object Reference") (`Hit Result` :type "HitResult Structure"))
  (message `/Game/DamageSystem/BPI_Damagable.TakeDamage` `Hit Actor` (make `/Game/DamageSystem/S_DamageInfo` (* Strength 10.0) "NewEnumerator2" "NewEnumerator1" false true false) self))

(fn `GetIdealRange`
  (returns (Attack :type "Float (double-precision)") (Defend :type "Float (double-precision)"))
  (return 600.0 600.0))

(fn `SetMovementSpeed`
  (params (Speed :type "/Game/New_AI/AI/Enums/E_MovementSpeed Enum" :default "NewEnumerator0"))
  (returns (SpeedValue :type "Float (double-precision)"))
  (set `CharacterMovementComponent.MaxWalkSpeed` (select `/Game/New_AI/AI/Enums/E_MovementSpeed` Speed :`NewEnumerator1` 400.0 :`NewEnumerator2` 500.0 :`NewEnumerator3` 500.0 :!type "Float (single-precision)") (`self.CharacterMovement`))
  (return 0.0))

(fn `UserConstructionScript`
  (`parent.UserConstructionScript`))