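; Sword-wielding enemy Blueprint that extends a parent enemy with weapon equip and melee attack behavior.
; Equip spawns a sword actor attached to the right-hand socket, and unequip destroys it, each notifying via dispatchers.
; Attack plays a slash montage that cannot be interrupted in the damage system until it ends.
; A montage notify runs a debug-drawn forward sphere trace, damages any pawn hit, and signals attack end.
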(event `self.ReceiveBeginPlay`
  (`parent.ReceiveBeginPlay`))

(event `/Game/New_AI/AI/BPI_EnemyAI.Attack`
  (bind _returnvalue (`self.K2_GetActorLocation`))
  (bind _notifyname (`|PlayMontage` (`self.Mesh`) "/Game/Animations/Melee/Montage_Sword_Slash.Montage_Sword_Slash")
    (:`then`
      (set `/Game/DamageSystem/BPC_DamageSystem.IsInterruptible` false (`self.BPC_DamageSystem`)))
    (:`OnCompleted`
      (`self.OnAttackEnd` :!label _label)
      (set `/Game/DamageSystem/BPC_DamageSystem.IsInterruptible` true (`self.BPC_DamageSystem`)))
    (:`OnInterrupted`
      (goto _label))
    (:`OnNotifyBegin`
      (switch `name` _notifyname
        (:`Slash`
          (bind (_outhit _returnvalue_2) (`KismetSystemLibrary.SphereTraceSingleForObjects` :`Start` _returnvalue :`End` (+ _returnvalue (* (`self.GetActorForwardVector`) (`self.BasicAttackRange`))) :`Radius` 20.0 :`ObjectTypes` (`|MakeArray` "ObjectTypeQuery3" :!type "EObjectTypeQuery Enum") :`DrawDebugType` "ForDuration"))
          (if _returnvalue_2
            (message `/Game/DamageSystem/BPI_Damagable.TakeDamage` (`.HitActor` (`GameplayStatics.BreakHitResult` _outhit)) (make `/Game/DamageSystem/S_DamageInfo` 25.0 "NewEnumerator1"))
            (`self.OnAttackEnd`)
            (else
              (`self.OnAttackEnd`))))))))

(event `/Game/New_AI/AI/BPI_EnemyAI.EquipWeapon`
  (bind _returnvalue (`|SpawnActorFromClass` "/Game/Weapons/BP_Base_Weapon_Sword.BP_Base_Weapon_Sword_C" (`self.GetTransform`) "Undefined" "MultiplyWithRoot" null null))
  (bind _output_get (set `self.WeaponRef` _returnvalue))
  (`self.K2_AttachToComponent` _output_get (`self.Mesh`) "hand_r_sword_socket" "SnapToTarget" "SnapToTarget" "SnapToTarget" true)
  (set `self.IsWeildingWeapon` true)
  (`self.OnWeaponEquiped`))

(event `/Game/New_AI/AI/BPI_EnemyAI.UnequipWeapon`
  (`self.K2_DestroyActor` (`self.WeaponRef`))
  (set `self.IsWeildingWeapon` false)
  (`self.OnWeaponUnequiped`))

(fn `UserConstructionScript`
  (`parent.UserConstructionScript`))