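; Ranged enemy base Blueprint that equips a rifle on BeginPlay and fires at its attack target.
; The spawned rifle attaches to a mesh socket, sets the wielding flag and calls the weapon-equipped event.
; Attack plays a fire montage whose notify triggers a BPCAttacks bullet trace toward the target, ending the attack on completion or interruption.
; It also defines movement speeds and ideal attack and defend ranges.
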(event `self.ReceiveBeginPlay`
  (`parent.ReceiveBeginPlay`)
  (`/Game/New_AI/AI/BPI_EnemyAI.EquipWeapon`))

(event `/Game/New_AI/AI/BPI_EnemyAI.EquipWeapon`
  (bind _returnvalue (`|SpawnActorFromClass` "/Game/Weapons/BP_Base_Weapon_Rifle.BP_Base_Weapon_Rifle_C" (`KismetMathLibrary.MakeTransform` (0.0 0.0 0.0)) "Undefined" "MultiplyWithRoot" null null))
  (bind _output_get (set `self.RifleRef` _returnvalue))
  (`self.K2_AttachToComponent` _output_get (`self.Mesh`) (`self.Socket NameKey`) "SnapToTarget" "SnapToTarget" "SnapToTarget" true)
  (set `self.IsWeildingWeapon` true)
  (`self.OnWeaponEquiped`))

(event `/Game/New_AI/AI/BPI_EnemyAI.Attack`
  (params (`Attack Target` :type "Actor Object Reference"))
  (`parent.Attack` `Attack Target`)
  (bind _notifyname (`|PlayMontage` (`self.Mesh`) "/Game/Animations/Rifle/Montage_Rifle_Fire.Montage_Rifle_Fire")
    (:`OnCompleted`
      (`/Game/New_AI/AI/BPI_EnemyAI.AttackEnd` `Attack Target` :!label _label))
    (:`OnInterrupted`
      (goto _label))
    (:`OnNotifyBegin`
      (switch `name` _notifyname
        (:`Fire`
          (`/Game/Attacks/BPC_Attacks.FireBullet` (`self.BPC_Attacks`) (`self.K2_GetActorLocation` (stale `/Game/New_AI/AI/BPI_EnemyAI.EquipWeapon` _output_get)) (`self.K2_GetActorLocation` `Attack Target`) (make `/Game/DamageSystem/S_DamageInfo` 15.0 "NewEnumerator2" "NewEnumerator0" false true)))))))

(fn `GetIdealRange`
  (returns (Attack :type "Float (double-precision)") (Defend :type "Float (double-precision)"))
  (return 600.0 600.0))

(fn `SetMovementSpeed`
  (params (Speed :type "/Game/New_AI/AI/Enums/E_MovementSpeed Enum" :default "NewEnumerator0"))
  (returns (SpeedValue :type "Float (double-precision)"))
  (set `CharacterMovementComponent.MaxWalkSpeed` (select `/Game/New_AI/AI/Enums/E_MovementSpeed` Speed :`NewEnumerator1` 200.0 :`NewEnumerator2` 300.0 :`NewEnumerator3` 500.0 :!type "Float (single-precision)") (`self.CharacterMovement`))
  (return 0.0))

(fn `UserConstructionScript`
  (`parent.UserConstructionScript`))