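; Base enemy character, handling health, damage, team, patrol route, movement speed and arced jump launches.
; BPCDamageSystem drives a widget health bar, ragdoll death and hit reactions that freeze the AIC_Enemy_Base controller, then resume attacking, targeting damage causers from other teams.
; Attacks reserve tokens from their target, track them per target and return them on attack end.
; The death loop's token return is unwired, so held tokens are not released there.
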(event `self.ReceiveBeginPlay`
  (bind _bpc_damagesystem (`self.BPC_DamageSystem`))
  (bind _asaic_enemy_base (cast `/Game/New_AI/AI/AIC_Enemy_Base` (`AIBlueprintHelperLibrary.GetAIController` self)))
  (set `self.AIC Enemy Base` _asaic_enemy_base)
  (bind _returnvalue (`|CreateWidget` "/Game/DamageSystem/W_HealthBar.W_HealthBar_C" null self))
  (`WidgetComponent.SetWidget` (`self.HealthBar`) _returnvalue)
  (add `/Game/DamageSystem/BPC_DamageSystem.OnDeath` _bpc_damagesystem (`|CreateDelegate` :!event `OnDeath_Event`))
  (add `/Game/DamageSystem/BPC_DamageSystem.OnDamageResponse` _bpc_damagesystem (`|CreateDelegate` :!event `Hit Response`)))

(event `OnDeath_Event`
  (bind _mesh (`self.Mesh`))
  (bind _aic_enemy_base (`self.AIC Enemy Base`))
  (`PrimitiveComponent.SetSimulatePhysics` _mesh true)
  (`PrimitiveComponent.SetCollisionEnabled` _mesh "QueryAndPhysics")
  (`BrainComponent.StopLogic` (`AIController.BrainComponent` _aic_enemy_base) "")
  (`/Game/New_AI/AI/AIC_Enemy_Base.SetStateAsDead` _aic_enemy_base)
  (bind _keys (`BlueprintMapLibrary.Map_Keys` (`self.Reserves Attack Tokens`)))
  (for _array_element _keys
    _))

(event `Hit Response`
  (params (DamageResponse :type "/Game/DamageSystem/E_DamageResponse Enum" :default "NewEnumerator0") (DamageCauser :type "Actor Object Reference"))
  (`MovementComponent.StopMovementImmediately` (`self.CharacterMovement`))
  (`/Game/New_AI/AI/AIC_Enemy_Base.SetStateAsFrozen` (`self.AIC Enemy Base`))
  (`|PlayMontage` (`self.Mesh`) (`self.HitRectionMontage`)
    (:`OnCompleted`
      _)
    (:`OnInterrupted`
      _))
  (bind _asaic_enemy_base (cast `/Game/New_AI/AI/AIC_Enemy_Base` (`self.GetController`)))
  (bind _teamnumber (message `/Game/DamageSystem/BPI_Damagable.GetTeamNumber` DamageCauser))
  (`/Game/New_AI/AI/AIC_Enemy_Base.SetStateAsAttacking` _asaic_enemy_base (select `bool` (!= (`self.Team Number`) _teamnumber) :`true` DamageCauser) true))

(event `/Game/New_AI/AI/BPI_EnemyAI.JumpToDestination`
  (params (Destination :type "Vector Structure"))
  (bind _outlaunchvelocity (`GameplayStatics.SuggestProjectileVelocity_CustomArc` (`self.K2_GetActorLocation`) (`KismetMathLibrary.MakeVector` Destination_X Destination_Y (+ Destination_Z 500.0))))
  (`self.LaunchCharacter` _outlaunchvelocity true true))

(event `/Game/DamageSystem/BPI_Damagable.Return Attack Token`
  (params (Amount :type Integer))
  (`/Game/DamageSystem/BPC_DamageSystem.Return Attack Token` (`self.BPC_DamageSystem`) Amount))

(event `/Game/New_AI/AI/BPI_EnemyAI.StoreAttackTokens`
  (params (`Attack Target` :type "Actor Object Reference") (Armount :type Integer))
  (bind (_value _returnvalue) (`BlueprintMapLibrary.Map_Find` (`self.Reserves Attack Tokens`) `Attack Target`))
  (`BlueprintMapLibrary.Map_Add` (`self.Reserves Attack Tokens`) `Attack Target` (`KismetMathLibrary.SelectInt` (+ Armount _value) Armount _returnvalue)))

(event `/Game/New_AI/AI/BPI_EnemyAI.AttackEnd`
  (params (AttackTarget :type "Actor Object Reference"))
  (bind _tokenusedincurrentattack (`self.TokenUsedInCurrentAttack`))
  (message `/Game/DamageSystem/BPI_Damagable.Return Attack Token` AttackTarget _tokenusedincurrentattack)
  (`/Game/New_AI/AI/BPI_EnemyAI.StoreAttackTokens` AttackTarget (* _tokenusedincurrentattack -1))
  (set `self.Attacking` false)
  (`self.OnAttackEnd`))

(event `/Game/New_AI/AI/BPI_EnemyAI.Attack`
  (params (`Attack Target` :type "Actor Object Reference"))
  (set `self.Attacking` true))

(event `/Game/DamageSystem/BPI_Damagable.SetIsInterupable`
  (params (Isinterruable :type Boolean))
  (set `/Game/DamageSystem/BPC_DamageSystem.IsInterruptible` Isinterruable (`self.BPC_DamageSystem`)))

(fn `AttackStart`
  (params (AttackTarget :type "Actor Object Reference") (Amount :type Integer))
  (returns (Sucess :type Boolean))
  (bind _sucess (message `/Game/DamageSystem/BPI_Damagable.Reserve Attack Token` AttackTarget Amount))
  (if _sucess
    (`/Game/New_AI/AI/BPI_EnemyAI.StoreAttackTokens` AttackTarget Amount)
    (set `self.TokenUsedInCurrentAttack` Amount)
    (return true)
    (else
      (return false))))

(fn `Get Movement Direction`
  (params (`input action` :type "InputAction Object Reference"))
  (returns (`Direction Key` :type "Key Structure"))
  (message `EnhancedInputSubsystemInterface.QueryKeysMappedToAction` (pcsubsystem `EnhancedInputLocalPlayerSubsystem` (`GameplayStatics.GetPlayerController` 0)) `input action`)
  (for _array_element _
    (if (`PlayerController.IsInputKeyDown` (`GameplayStatics.GetPlayerController` 0) _array_element)
      (return _array_element))))

(fn `GetCurrentHealth`
  (returns (Health :type "Float (double-precision)"))
  (return (`/Game/DamageSystem/BPC_DamageSystem.Health` (`self.BPC_DamageSystem`))))

(fn `GetIdealRange`
  (returns (Attack :type "Float (double-precision)") (Defend :type "Float (double-precision)"))
  (return 150.0 350.0))

(fn `GetMaxHealth`
  (returns (MaxHealth :type "Float (double-precision)"))
  (return (`/Game/DamageSystem/BPC_DamageSystem.MaxHealth` (`self.BPC_DamageSystem`))))

(fn `GetPatrolRoute`
  (returns (PatrolRoute :type "/Game/New_AI/AI/BP_PatrolRoute Object Reference"))
  (return (`self.PatrolRoute`)))

(fn `GetTeamNumber`
  (returns (TeamNumber :type Integer))
  (return (`self.Team Number`)))

(fn `Heal`
  (params (Amount :type "Float (double-precision)"))
  (returns (NewHealth :type "Float (double-precision)"))
  (bind _newhealth (`/Game/DamageSystem/BPC_DamageSystem.Heal` (`self.BPC_DamageSystem`) Amount))
  (return _newhealth))

(fn `IsAttacking`
  (returns (Attacking :type Boolean))
  (return (`self.Attacking`)))

(fn `IsDead`
  (returns (Dead :type Boolean))
  (return (`/Game/DamageSystem/BPC_DamageSystem.IsDead` (`self.BPC_DamageSystem`))))

(fn `Reserve Attack Token`
  (params (Amount :type Integer))
  (returns (Sucess :type Boolean))
  (bind _sucess (`/Game/DamageSystem/BPC_DamageSystem.Reserve Attack Token` (`self.BPC_DamageSystem`) Amount))
  (return _sucess))

(fn `SetMovementSpeed`
  (params (Speed :type "/Game/New_AI/AI/Enums/E_MovementSpeed Enum" :default "NewEnumerator0"))
  (returns (SpeedValue :type "Float (double-precision)"))
  (bind _output_get (set `CharacterMovementComponent.MaxWalkSpeed` (select `/Game/New_AI/AI/Enums/E_MovementSpeed` Speed :`NewEnumerator1` 100.0 :`NewEnumerator2` 300.0 :`NewEnumerator3` 500.0 :!type "Float (single-precision)") (`self.CharacterMovement`)))
  (return _output_get))

(fn `TakeDamage`
  (params (DamageInfo :type "/Game/DamageSystem/S_DamageInfo Structure") (`Damage Causer` :type "Actor Object Reference"))
  (returns (WasDamaged :type Boolean))
  (bind _wasdamaged (`/Game/DamageSystem/BPC_DamageSystem.TakeDamage` (`self.BPC_DamageSystem`) DamageInfo `Damage Causer`))
  (return _wasdamaged))

(fn `UserConstructionScript`)