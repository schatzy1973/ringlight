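; Zombie enemy Blueprint that wields a sword and offers a short-range slash and a ground smash attack.
; Equipping spawns the sword on a hand socket and signals completion, while unequipping destroys it.
; Attack events pass montage and damage info to the BPCAttacks component, with the slash blockable and parryable and the smash applying an area status effect.
; Helpers report ideal attack and defend ranges and linearly predict an actor's future position from horizontal velocity.
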(event `self.ReceiveBeginPlay`
  ;[1 1 1] BeginPlay
  (`parent.ReceiveBeginPlay`))

(event `self.EquipWeapon`
  ;[1 1 1] Equip Weapon
  (bind _returnvalue (`|SpawnActorFromClass` "/Game/Weapons/BP_Base_Weapon_Sword.BP_Base_Weapon_Sword_C" (`self.GetTransform`) "Undefined" "MultiplyWithRoot" null null))
  (bind _output_get (set `self.WeaponRef` _returnvalue))
  (`self.K2_AttachToComponent` _output_get (`self.Mesh`) "hand_r_sword_socket" "SnapToTarget" "SnapToTarget" "SnapToTarget" true)
  (set `self.IsWeildingWeapon` true)
  (`self.OnWeaponEquiped`))

(event `ShortRangeAttack`
  (params (AttackTarget :type "Actor Object Reference"))
  ;[1 1 1] Basic Attack
  (`/Game/Attacks/BPC_Attacks.PrimaryMeleeAttack` (`self.BPC_Attacks`) (make `/Game/Attacks/S_AttackInfo` AttackTarget "/Game/Animations/Melee/Montage_Sword_Slash.Montage_Sword_Slash" (make `/Game/DamageSystem/S_DamageInfo` 10.0 "NewEnumerator1" "NewEnumerator0" false true true)) 200.0 20.0)
  (`KismetSystemLibrary.PrintString` "Hello"))

(event `self.UnequipWeapon`
  ;[1 1 1] Unequip Weapon
  (`self.K2_DestroyActor` (`self.WeaponRef`))
  (set `self.IsWeildingWeapon` false))

(event `GroundSmashAttack`
  (params (`Attack Target` :type "Actor Object Reference"))
  ;[1 1 1] Basic Attack
  (`/Game/Attacks/BPC_Attacks.Ground Smash` (`self.BPC_Attacks`) (make `/Game/Attacks/S_AttackInfo` `Attack Target` "/Game/Animations/Melee/Montage_Melee_GroundSmash.Montage_Melee_GroundSmash" (make `/Game/DamageSystem/S_DamageInfo` 15.0 "NewEnumerator3")) 300.0 "NewEnumerator0"))

(event `CustomEvent`
  (params (`Attack Target` :type "Actor Object Reference"))
  ;[1 1 1] Basic Attack
)

(fn `CalculateFutureActorLocation`
  (params (Actor :type "Actor Object Reference") (Time :type "Float (double-precision)" :default 1.0))
  (returns (Location :type "Vector Structure"))
  (return (+ (`self.K2_GetActorLocation` Actor) (* (* (`self.GetVelocity` Actor) (1.0 1.0 0.0)) Time))))

(fn `GetIdealRange`
  (returns (Attack :type "Float (double-precision)") (Defend :type "Float (double-precision)"))
  (return 200.0 400.0))

(fn `UserConstructionScript`
  (`parent.UserConstructionScript`))