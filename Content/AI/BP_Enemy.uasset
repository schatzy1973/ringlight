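; Melee enemy character with sword combo and big-attack montages, a stats-driven health bar and ragdoll death.
; Incoming damage reduces a BPCStats value, and HealthCollision overlap shows or hides the bar widget for the player.
; Begin/EndSwordTrace toggle a looping timer that sphere-traces between blade points, with DoOnce plus Delay throttling hits.
; PointDamageTrace applies radial slam damage to one pawn, while DIe disables movement and removes the widget.
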(event `self.ReceiveBeginPlay`
  (bind _aswb_enermy_health (cast `/Game/Souls/Blueprints/WB_EnermyHealth` (`WidgetComponent.GetWidget` (`self.Widget`))))
  (`/Game/Souls/Blueprints/BPC_Stats.Set Health Progress bar` (`self.BPC_Stats`) (`/Game/Souls/Blueprints/WB_EnermyHealth.HealthBar` _aswb_enermy_health)))

(event `self.ReceiveAnyDamage`
  (params (Damage :type "Float (single-precision)") (DamageType :type "DamageType Object Reference") (InstigatedBy :type "Controller Object Reference") (DamageCauser :type "Actor Object Reference"))
  (`/Game/Souls/Blueprints/BPC_Stats.Increase value` (`self.BPC_Stats`) "NewEnumerator0" (* Damage -1.0)))

(event `/Game/Souls/Blueprints/BPI_DMG.End Sword Trace`
  ;[1 1 1] Sword Traces
  (if (`KismetSystemLibrary.K2_IsValidTimerHandle` (stale `/Game/Souls/Blueprints/BPI_DMG.BeginSword Trace` _returnvalue))
    (`KismetSystemLibrary.K2_ClearAndInvalidateTimerHandle` (stale `/Game/Souls/Blueprints/BPI_DMG.BeginSword Trace` _returnvalue))))

(event `/Game/Souls/Blueprints/BPI_DMG.BeginSword Trace`
  ;[1 1 1] Sword Traces
  (bind _returnvalue (`KismetSystemLibrary.K2_SetTimerDelegate` (delegate `Damage_Trace`) 0.1 true)))

(event `Damage_Trace`
  ;[1 1 1] Sword Traces
  (if (not (`self.Isdead`))
    (bind (_outhit _returnvalue) (`KismetSystemLibrary.SphereTraceSingleForObjects` :`Start` (`SceneComponent.K2_GetComponentLocation` (`self.StartTrace`)) :`End` (`SceneComponent.K2_GetComponentLocation` (`self.EndTrace`)) :`Radius` 25.0 :`ObjectTypes` (`|MakeArray` "ObjectTypeQuery3" :!type "EObjectTypeQuery Enum") :`DrawDebugType` "ForOneFrame"))
    (if _returnvalue
      (`/Engine/EditorBlueprintResources/StandardMacros.DoOnce` false :!label _label
        (:`Completed`
          (`GameplayStatics.PlaySound2D` "/Game/Sounds/163441__under7dude__man-getting-hit.163441__under7dude__man-getting-hit" 1.0 1.0 0.0 null null)
          (`GameplayStatics.ApplyDamage` (`.HitActor` (`GameplayStatics.BreakHitResult` _outhit)) (`self.Damage`))
          (`KismetSystemLibrary.Delay` 0.3)
          (goto _label :!via `Reset`))))))

(event `/Game/Souls/Blueprints/BPI_DMG.DIe`
  (`CharacterMovementComponent.DisableMovement` (`self.CharacterMovement`))
  (`PrimitiveComponent.SetSimulatePhysics` (`self.Mesh`) true)
  (set `self.Isdead` true)
  (`ActorComponent.K2_DestroyComponent` (`self.Widget`)))

(event `/Game/Souls/Blueprints/BPI_DMG.Point Damage Trace`
  (bind _returnvalue (`SceneComponent.K2_GetComponentLocation` (`self.Point Trace pos`)))
  (bind (_outhit _returnvalue_2) (`KismetSystemLibrary.SphereTraceSingleForObjects` :`Start` _returnvalue :`End` _returnvalue :`Radius` (`self.Slam radius`) :`ObjectTypes` (`|MakeArray` "ObjectTypeQuery3" :!type "EObjectTypeQuery Enum") :`DrawDebugType` "ForDuration"))
  (if _returnvalue_2
    (`GameplayStatics.ApplyDamage` (`.HitActor` (`GameplayStatics.BreakHitResult` _outhit)) (`self.Slam Damage`))))

(event `self.HealthCollision.OnComponentBeginOverlap`
  (params (OverlappedComponent :type "PrimitiveComponent Object Reference") (OtherActor :type "Actor Object Reference") (OtherComp :type "PrimitiveComponent Object Reference") (OtherBodyIndex :type Integer) (bFromSweep :type Boolean) (SweepResult :type "HitResult Structure (by ref)"))
  (cast `/Game/ThirdPerson/Blueprints/BP_ThirdPersonCharacter` OtherActor)
  (`SceneComponent.SetVisibility` (`self.Widget`) true false))

(event `self.HealthCollision.OnComponentEndOverlap`
  (params (OverlappedComponent :type "PrimitiveComponent Object Reference") (OtherActor :type "Actor Object Reference") (OtherComp :type "PrimitiveComponent Object Reference") (OtherBodyIndex :type Integer))
  (cast `/Game/ThirdPerson/Blueprints/BP_ThirdPersonCharacter` OtherActor)
  (`SceneComponent.SetVisibility` (`self.Widget`) false false))

(fn `BigAttack`
  (returns (Duration :type "Float (double-precision)"))
  (bind _returnvalue (`self.PlayAnimMontage` "/Game/Souls/Combat/Combat_Animations/BigAttack_Montage.BigAttack_Montage"))
  (return _returnvalue))

(fn `SwordAttack`
  (returns (AnimDuration :type "Float (double-precision)"))
  (bind _returnvalue (`self.PlayAnimMontage` "/Game/Souls/Combat/Combat_Animations/SwordAttackCombo_Montage.SwordAttackCombo_Montage"))
  (return _returnvalue))

(fn `UserConstructionScript`)