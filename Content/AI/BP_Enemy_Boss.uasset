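; Boss enemy character that opens the way out of the level by spawning an exit when it dies.
; Its death event disables movement, ragdolls the mesh through physics simulation, sets the dead flag and hides the widget component.
; After a short delay, it spawns BP_Exit_ at the boss's current location.
; The graph adds no other active logic, as BeginPlay, overlap and Tick are unused stubs.
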(event `/Game/Souls/Blueprints/BPI_DMG.DIe`
  (`CharacterMovementComponent.DisableMovement` (`self.CharacterMovement`))
  (`PrimitiveComponent.SetSimulatePhysics` (`self.Mesh`) true)
  (set `self.Isdead` true)
  (`SceneComponent.SetVisibility` (`self.Widget`) false false)
  (`KismetSystemLibrary.Delay` 0.2)
  (`|SpawnActorFromClass` "/Game/Dungeon/BP_Exit_.BP_Exit__C" (`KismetMathLibrary.MakeTransform` (`self.K2_GetActorLocation`)) "Undefined" "MultiplyWithRoot" null null))

(fn `UserConstructionScript`
  (`parent.UserConstructionScript`))