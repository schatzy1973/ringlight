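; Player combat component for a souls-like third-person character, handling target lock, sword attacks and dodging.
; Lock-on sphere-traces from the camera, attaches a marker actor and turns the controller toward the target each tick.
; Attack and dodge montages spend stamina and pause its regeneration; notifies check a combo flag, and locked dodges follow the direction key.
; Externally triggered events run a looping timer sphere trace along the sword, applying damage through a resetting DoOnce.
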(event `self.ReceiveTick`
  (params (DeltaSeconds :type "Float (single-precision)"))
  (`|ExecutionSequence`
    (:`then_0`
      (`self.TargetLockTick`))))

(event `self.ReceiveBeginPlay`
  (bind _asbp_third_person_character (cast `/Game/ThirdPerson/Blueprints/BP_ThirdPersonCharacter` (`self.GetOwner`)))
  (set `self.PlayerRef` _asbp_third_person_character))

(event `EnhancedInput|/Game/ThirdPerson/Input/Actions/IA_Lock`
  (params (ActionValue :type "Vector2D Structure") (ElapsedSeconds :type "Float (double-precision)") (TriggeredSeconds :type "Float (double-precision)") (InputAction :type "InputAction Object Reference" :default "/Game/ThirdPerson/Input/Actions/IA_Lock.IA_Lock"))
  (bind _returnvalue (`Actor.GetTransform` (`self.Target lock Actor`)))
  (bind _transformcomponent (`PlayerCameraManager.TransformComponent` (`GameplayStatics.GetPlayerCameraManager` 0)))
  (bind _charactermovement (`Character.CharacterMovement` (`self.PlayerRef`)))
  (bind _charactermovement_2 (`Character.CharacterMovement` (`self.PlayerRef`)))
  (bind (_returnvalue_x _returnvalue_y _returnvalue_z) (`KismetMathLibrary.BreakVector` (`SceneComponent.K2_GetComponentLocation` _transformcomponent)))
  ;[1 1 1] Target Lock
  (:`Started`
    (`self.Target lock Actor`
      (:`then`
        (set `self.Target lock Actor` null)
        (set `CharacterMovementComponent.bOrientRotationToMovement` true _charactermovement)
        (set `CharacterMovementComponent.bUseControllerDesiredRotation` false _charactermovement)
        (`Actor.K2_DestroyActor` (`self.Targetlock Widget`))
        (set `self.IsLocking` false))
      (:`else`
        (bind (_outhit _returnvalue_2) (`KismetSystemLibrary.SphereTraceSingleForObjects` (`KismetMathLibrary.MakeVector` _returnvalue_x _returnvalue_y _returnvalue_z) (+ (`KismetMathLibrary.MakeVector` _returnvalue_x _returnvalue_y (+ _returnvalue_z 20.0)) (* (`KismetMathLibrary.GetForwardVector` (`SceneComponent.K2_GetComponentRotation` _transformcomponent)) 1000.0)) 50.0 (`|MakeArray` "ObjectTypeQuery3" :!type "EObjectTypeQuery Enum")))
        (if _returnvalue_2
          (bind (_bblockinghit _binitialoverlap _time _distance _location _impactpoint _normal _impactnormal _physmat _hitactor) (`GameplayStatics.BreakHitResult` _outhit))
          (if (not (`Actor.ActorHasTag` _hitactor "Hero"))
            (set `self.Target lock Actor` _hitactor)
            (set `CharacterMovementComponent.bOrientRotationToMovement` false _charactermovement_2)
            (set `CharacterMovementComponent.bUseControllerDesiredRotation` true _charactermovement_2)
            (bind _returnvalue_3 (`|SpawnActorFromClass` "/Game/Souls/Blueprints/BP_TargetLock_Widget.BP_TargetLock_Widget_C" (`KismetMathLibrary.MakeTransform` (`KismetMathLibrary.MakeVector` (.x (.location _returnvalue)) (.y (.location _returnvalue)) (+ (.z (.location _returnvalue)) 20.0)) (.rotation _returnvalue)) "AlwaysSpawn" "MultiplyWithRoot" null null))
            (bind _output_get (set `self.Targetlock Widget` _returnvalue_3))
            (`Actor.K2_AttachToActor` _output_get (`self.Target lock Actor`) "None" "SnapToTarget" "SnapToTarget" "SnapToTarget" true)
            (set `self.IsLocking` true)))))))

(event `EnhancedInput|/Game/ThirdPerson/Input/Actions/IA_Attack`
  (params (ActionValue :type "Vector2D Structure") (ElapsedSeconds :type "Float (double-precision)") (TriggeredSeconds :type "Float (double-precision)") (InputAction :type "InputAction Object Reference" :default "/Game/ThirdPerson/Input/Actions/IA_Attack.IA_Attack"))
  (bind _bpc_stats (`/Game/ThirdPerson/Blueprints/BP_ThirdPersonCharacter.BPC_Stats` (`self.PlayerRef`)))
  (bind _bpc_stats_2 (`/Game/ThirdPerson/Blueprints/BP_ThirdPersonCharacter.BPC_Stats` (`self.PlayerRef`)))
  ;[1 1 1] Sword Combo Animation
  (:`Started`
    (if (and (not (`self.Is Attacking`)) (>= (`/Game/Souls/Blueprints/BPC_Stats.Stamina` (`/Game/ThirdPerson/Blueprints/BP_ThirdPersonCharacter.BPC_Stats` (`self.PlayerRef`))) 10.0))
      (set `self.Is Attacking` true)
      (`|PlayMontage` (`Character.Mesh` (`self.PlayerRef`)) "/Game/Souls/Combat/Combat_Animations/SwordAttackCombo_Montage.SwordAttackCombo_Montage"
        (:`then`
          (set `/Game/Souls/Blueprints/BPC_Stats.RegainStamina` false _bpc_stats_2)
          (`/Game/Souls/Blueprints/BPC_Stats.Increase value` _bpc_stats_2 "NewEnumerator1" -10.0))
        (:`OnCompleted`
          (set `self.Is Attacking` false :!label _label)
          (set `self.Combo?` false)
          (set `/Game/Souls/Blueprints/BPC_Stats.RegainStamina` true _bpc_stats))
        (:`OnInterrupted`
          (goto _label))
        (:`OnNotifyBegin`
          (if (and (`self.Is Attacking`) (`self.Combo?`))
            (set `self.Combo?` false)
            (`/Game/Souls/Blueprints/BPC_Stats.Increase value` _bpc_stats "NewEnumerator1" -10.0)
            (else
              (`AnimInstance.Montage_Stop` (`SkeletalMeshComponent.GetAnimInstance` (`Character.Mesh` (`self.PlayerRef`))) 0.2 "/Game/Souls/Combat/Combat_Animations/SwordAttackCombo_Montage.SwordAttackCombo_Montage")))))
      (else
        (set `self.Combo?` false)))))

(event `End Damage Trace`
  ;[1 1 1] Sword Traces
  (if (`KismetSystemLibrary.K2_IsValidTimerHandle` (stale `Begin_Dmg_Trace` _returnvalue))
    (`KismetSystemLibrary.K2_ClearAndInvalidateTimerHandle` (stale `Begin_Dmg_Trace` _returnvalue))))

(event `Begin_Dmg_Trace`
  ;[1 1 1] Sword Traces
  (bind _returnvalue (`KismetSystemLibrary.K2_SetTimerDelegate` (delegate `Damage_Trace`) 0.1 true)))

(event `Damage_Trace`
  (bind _playerref (`self.PlayerRef`))
  ;[1 1 1] Sword Traces
  (bind (_outhit _returnvalue) (`KismetSystemLibrary.SphereTraceSingleForObjects` :`Start` (`SceneComponent.K2_GetComponentLocation` (`/Game/ThirdPerson/Blueprints/BP_ThirdPersonCharacter.StartTrace` _playerref)) :`End` (`SceneComponent.K2_GetComponentLocation` (`/Game/ThirdPerson/Blueprints/BP_ThirdPersonCharacter.EndTrace` _playerref)) :`Radius` 100.0 :`ObjectTypes` (`|MakeArray` "ObjectTypeQuery3" :!type "EObjectTypeQuery Enum") :`DrawDebugType` "ForOneFrame"))
  (if _returnvalue
    (`/Engine/EditorBlueprintResources/StandardMacros.DoOnce` false :!label _label_2
      (:`Completed`
        (`GameplayStatics.PlaySound2D` "/Game/Sounds/163441__under7dude__man-getting-hit.163441__under7dude__man-getting-hit" 1.0 1.0 0.0 null null)
        (`GameplayStatics.ApplyDamage` (`.HitActor` (`GameplayStatics.BreakHitResult` _outhit)) (`self.Damage`))
        (`KismetSystemLibrary.Delay` 0.3)
        (goto _label_2 :!via `Reset`)))))

(event `EnhancedInput|/Game/ThirdPerson/Input/Actions/IA_dodge`
  (params (ActionValue :type Boolean) (ElapsedSeconds :type "Float (double-precision)") (TriggeredSeconds :type "Float (double-precision)") (InputAction :type "InputAction Object Reference" :default "/Game/ThirdPerson/Input/Actions/IA_dodge.IA_dodge"))
  (bind _bpc_stats (`/Game/ThirdPerson/Blueprints/BP_ThirdPersonCharacter.BPC_Stats` (`self.PlayerRef`)))
  ;[1 1 1] Dodging
  (:`Started`
    (if (and (not (`self.Is Dodging?`)) (>= (`/Game/Souls/Blueprints/BPC_Stats.Stamina` (`/Game/ThirdPerson/Blueprints/BP_ThirdPersonCharacter.BPC_Stats` (`self.PlayerRef`))) 25.0))
      (set `self.Is Dodging?` true)
      (`|ExecutionSequence`
        (:`then_0`
          (if (`CharacterMovementComponent.bUseControllerDesiredRotation` (`Character.CharacterMovement` (`self.PlayerRef`)))
            (switch `string` (`KismetTextLibrary.Conv_TextToString` (`KismetInputLibrary.Key_GetDisplayName` (`/Game/ThirdPerson/Blueprints/BP_ThirdPersonCharacter.Direction Key` (`self.PlayerRef`))))
              (:`W`
                (set `self.Direction` "NewEnumerator0"))
              (:`S`
                (set `self.Direction` "NewEnumerator1"))
              (:`A`
                (set `self.Direction` "NewEnumerator2"))
              (:`D`
                (set `self.Direction` "NewEnumerator3")))
            (else
              (set `self.Direction` "NewEnumerator0"))))
        (:`then_1`
          (`|PlayMontage` (`Character.Mesh` (`self.PlayerRef`)) (select `/Game/Souls/Blueprints/E_Direction` (`self.Direction`) :`NewEnumerator0` "/Game/Souls/Combat/Combat_Animations/Dodge/Dodge_F_Montage.Dodge_F_Montage" :`NewEnumerator1` "/Game/Souls/Combat/Combat_Animations/Dodge/Dodge_B_Montage.Dodge_B_Montage" :`NewEnumerator2` "/Game/Souls/Combat/Combat_Animations/Dodge/Dodge_L_Montage.Dodge_L_Montage" :`NewEnumerator3` "/Game/Souls/Combat/Combat_Animations/Dodge/Dodge_R_Montage.Dodge_R_Montage" :!type "AnimMontage Object Reference")
            (:`then`
              (set `/Game/Souls/Blueprints/BPC_Stats.RegainStamina` false (`/Game/ThirdPerson/Blueprints/BP_ThirdPersonCharacter.BPC_Stats` (`self.PlayerRef`)))
              (`/Game/Souls/Blueprints/BPC_Stats.Increase value` _bpc_stats "NewEnumerator1" -25.0))
            (:`OnCompleted`
              (set `self.Is Dodging?` false :!label _label_3)
              (set `/Game/Souls/Blueprints/BPC_Stats.RegainStamina` true _bpc_stats))
            (:`OnInterrupted`
              (goto _label_3))))))))