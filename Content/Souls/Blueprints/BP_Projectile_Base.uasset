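; Base projectile actor that flies at a set speed and gravity, with optional homing on a Target.
; The construction script configures ProjectileMovement and homing from its variables.
; On BeginPlay, only with a valid Target, it aims its velocity at that Target and makes the box collision ignore its instigator, or owner as fallback.
; On hit it fires the OnProjectileImpact dispatcher, spawns impact effect and sound, then destroys itself.
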(event `self.ReceiveBeginPlay`
  (bind _returnvalue (`self.GetInstigator`))
  (`self.Target`
    (:`then`
      (`self.Rotate To target`)
      (`PrimitiveComponent.IgnoreActorWhenMoving` (`self.BoxCollision`) (select `bool` (`KismetSystemLibrary.IsValid` _returnvalue) :`false` (`self.GetOwner`) :`true` _returnvalue :!type "Actor Object Reference") true))
    (:`else`)))

(event `Rotate To target`
  (`self.Target`
    (:`then`
      (set `MovementComponent.Velocity` (* (`KismetMathLibrary.GetDirectionUnitVector` (`self.K2_GetActorLocation`) (`self.K2_GetActorLocation` (`self.Target`))) (`self.Speed`)) (`self.ProjectileMovement`)))
    (:`else`)))

(event `self.BoxCollision.OnComponentHit`
  (params (HitComponent :type "PrimitiveComponent Object Reference") (OtherActor :type "Actor Object Reference") (OtherComp :type "PrimitiveComponent Object Reference") (NormalImpulse :type "Vector Structure") (Hit :type "HitResult Structure (by ref)"))
  (bind (_bblockinghit _binitialoverlap _time _distance _location) (`GameplayStatics.BreakHitResult` Hit))
  (`self.OnprojectileImpact` OtherActor Hit)
  (`GameplayStatics.SpawnEmitterAtLocation` (`self.impact effect`) _location)
  (`GameplayStatics.PlaySoundAtLocation` (`self.Impact sound`) _location (struct) 1.0 1.0 0.0 null null null null)
  (`self.K2_DestroyActor`))

(fn `UserConstructionScript`
  (bind _projectilemovement (`self.ProjectileMovement`))
  (bind _speed (`self.Speed`))
  (set `ProjectileMovementComponent.InitialSpeed` _speed _projectilemovement)
  (set `ProjectileMovementComponent.MaxSpeed` _speed _projectilemovement)
  (set `ProjectileMovementComponent.ProjectileGravityScale` (`self.Gravity`) _projectilemovement)
  (`self.Target`
    (:`then`
      (if (`self.is homing`)
        (set `ProjectileMovementComponent.bIsHomingProjectile` true _projectilemovement)
        (set `ProjectileMovementComponent.HomingTargetComponent` (`Actor.RootComponent` (`self.Target`)) _projectilemovement)))
    (:`else`)))