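; BPC_Stats is a stats component that tracks its owning actor's health and triggers death when it runs out.
; IncreaseValue switches on the given stat, adds the value to Health and clamps it between zero and MaxHealth.
; At zero it fires Die, which sends DIeMessage to the owner.
; It also updates an optional health progress bar, supplied through SetHealthProgressbar, with the health ratio.
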(event `Die`
  (message `/Game/Souls/Blueprints/BPI_DMG.DIe` (`self.GetOwner`)))

(event `Set Health Progress bar`
  (params (`HeathProgress bar` :type "ProgressBar Object Reference"))
  (set `self.Heath Progress Bar` `HeathProgress bar`))

(fn `Increase value`
  (params (stat :type "/Game/Souls/Blueprints/E_Stats Enum" :default "NewEnumerator0") (Value :type "Float (double-precision)"))
  (switch `/Game/Souls/Blueprints/E_Stats` stat
    (:`NewEnumerator0`
      (set `self.Health` (`KismetMathLibrary.FClamp` (+ (`self.Health`) Value) 0.0 (`self.Max Health`)))
      (`|ExecutionSequence`
        (:`then_0`
          (if (<= (`self.Health`) 0.0)
            (`self.Die`)))
        (:`then_1`
          (bind _heath_progress_bar (`self.Heath Progress Bar`)
            (:`then`
              (`ProgressBar.SetPercent` _heath_progress_bar (/ (`self.Health`) (`self.Max Health`))))
            (:`else`)))))))