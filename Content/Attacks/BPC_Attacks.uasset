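; Attack component that gives its owning character a library of melee, magic, bullet and leap attacks that damage only other teams.
; Most attacks play a montage whose notifies fire sphere traces, AOE actors or spawned projectiles, then message the owner when finished, often toggling interruptibility; bullets use a line trace.
; The leap predicts the target's position from its velocity and launches along a distance-scaled arc, stopping movement on landing.
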(event `Ground Smash`
  (params (`Attack Info` :type "/Game/Attacks/S_AttackInfo Structure") (Radius :type "Float (double-precision)") (`Status Effect` :type "/Game/AOE/E_StatusEffect Enum" :default "NewEnumerator0"))
  (bind (_attacktarget _montage _damageinfo) (break `/Game/Attacks/S_AttackInfo` `Attack Info`))
  (bind _returnvalue (`self.GetOwner`))
  ;[1 1 1] Melee Attacks
  (bind _mesh (`self.AttackBase` _attacktarget))
  (bind _notifyname (`|PlayMontage` _mesh _montage)
    (:`then`
      (message `/Game/DamageSystem/BPI_Damagable.SetIsInterupable` _returnvalue false))
    (:`OnCompleted`
      (message `/Game/New_AI/AI/BPI_EnemyAI.AttackEnd` _returnvalue _attacktarget :!label _label)
      (message `/Game/DamageSystem/BPI_Damagable.SetIsInterupable` _returnvalue true))
    (:`OnInterrupted`
      (goto _label))
    (:`OnNotifyBegin`
      (switch `name` _notifyname
        (:`Smash`
          (`self.AOEDamage` Radius _damageinfo `Status Effect`))))))

(event `Basic Mage Spell`
  (params (`Attack Info` :type "/Game/Attacks/S_AttackInfo Structure"))
  (bind (_attacktarget _montage _damageinfo) (break `/Game/Attacks/S_AttackInfo` `Attack Info`))
  ;[1 1 1] Magic Spells
  (bind _mesh (`self.AttackBase` _attacktarget))
  (bind _notifyname (`|PlayMontage` _mesh _montage)
    (:`OnCompleted`
      (message `/Game/New_AI/AI/BPI_EnemyAI.AttackEnd` (`self.GetOwner`) _attacktarget :!label _label_2))
    (:`OnInterrupted`
      (goto _label_2))
    (:`OnNotifyBegin`
      (switch `name` _notifyname
        (:`Fire`
          (`self.Magic Spell` (`KismetMathLibrary.MakeTransform` (`SceneComponent.GetSocketLocation` _mesh "RightHand")) _attacktarget _damageinfo))))))

(event `Magic Spell`
  (params (SpawnTransform :type "Transform Structure") (Target :type "Actor Object Reference") (DamageInfo :type "/Game/DamageSystem/S_DamageInfo Structure") (Alt :type Boolean))
  ;[1 1 1] Attack Notifys
  ;;[0 0 0] Basic Magic Spell
  (bind _returnvalue (`|SpawnActorFromClass` (select `bool` Alt :`false` "/Game/Projectiles/BP_Projectile_DarkEnergy.BP_Projectile_DarkEnergy_C" :`true` "/Game/Projectiles/BP_Projectile_DarkEnergy_Alt.BP_Projectile_DarkEnergy_Alt_C" :!type "/Game/Projectiles/BP_Projectile_Base Class Reference") SpawnTransform "Undefined" "MultiplyWithRoot" (`self.GetOwner`) 1000.0 0.0 Target false null))
  (add `/Game/Projectiles/BP_Projectile_Base.OnProjectileImpact` _returnvalue (delegate `OnProjectileImpact_Event`))
  (`PrimitiveComponent.IgnoreActorWhenMoving` (`Actor.GetComponentByClass` (`self.GetOwner`) "/Script/Engine.CapsuleComponent") _returnvalue true))

(event `OnProjectileImpact_Event`
  (params (OtherActor :type "Actor Object Reference") (Hit :type "HitResult Structure"))
  (bind _returnvalue (`self.GetOwner`))
  ;[1 1 1] Attack Notifys
  ;;[0 0 0] Basic Magic Spell
  (message `/Game/DamageSystem/BPI_Damagable.TakeDamage` OtherActor (stale `Magic Spell` DamageInfo) _returnvalue "NewEnumerator0")
  (`AISense_Damage.ReportDamageEvent` OtherActor _returnvalue (`.Amount_2_64864A0D4320D27C3EA14D8019B5EC9D` (break `/Game/DamageSystem/S_DamageInfo` (stale `Magic Spell` DamageInfo))) (`Actor.K2_GetActorLocation` (`self.GetOwner`)))
  (`self.OnAttackEnded`))

(event `BarrageSpell`
  (params (`Attack Info` :type "/Game/Attacks/S_AttackInfo Structure"))
  (bind (_attacktarget _montage _damageinfo) (break `/Game/Attacks/S_AttackInfo` `Attack Info`))
  (bind _returnvalue (`self.GetOwner`))
  ;[1 1 1] Magic Spells
  (bind _mesh (`self.AttackBase` _attacktarget))
  (bind _notifyname (`|PlayMontage` _mesh _montage)
    (:`OnCompleted`
      (message `/Game/New_AI/AI/BPI_EnemyAI.AttackEnd` _returnvalue _attacktarget :!label _label_3)
      (message `/Game/DamageSystem/BPI_Damagable.SetIsInterupable` _returnvalue true))
    (:`OnInterrupted`
      (goto _label_3))
    (:`OnNotifyBegin`
      (switch `name` _notifyname
        (:`Fire`
          (`self.Magic Spell` (`KismetMathLibrary.MakeTransform` (`SceneComponent.GetSocketLocation` _mesh "RightHand") (`KismetMathLibrary.FindLookAtRotation` (`Actor.K2_GetActorLocation` (`self.GetOwner`)) (+ (`Actor.K2_GetActorLocation` _attacktarget) (`KismetMathLibrary.MakeVector` 0.0 (`KismetMathLibrary.RandomFloatInRange` -300.0 300.0))))) null _damageinfo true)
          (message `/Game/DamageSystem/BPI_Damagable.SetIsInterupable` _returnvalue false))))))

(event `PrimaryMeleeAttack`
  (params (AttackInfo :type "/Game/Attacks/S_AttackInfo Structure") (Length :type "Float (double-precision)") (Radius :type "Float (single-precision)"))
  (bind (_attacktarget _montage _damageinfo) (break `/Game/Attacks/S_AttackInfo` AttackInfo))
  (bind _returnvalue (`self.GetOwner`))
  ;[1 1 1] Melee Attacks
  (bind _mesh (`self.AttackBase` _attacktarget))
  (bind _notifyname (`|PlayMontage` _mesh _montage)
    (:`then`
      (message `/Game/DamageSystem/BPI_Damagable.SetIsInterupable` _returnvalue false))
    (:`OnCompleted`
      (message `/Game/New_AI/AI/BPI_EnemyAI.AttackEnd` _returnvalue _attacktarget :!label _label_4)
      (message `/Game/DamageSystem/BPI_Damagable.SetIsInterupable` _returnvalue true))
    (:`OnInterrupted`
      (goto _label_4))
    (:`OnNotifyBegin`
      (switch `name` _notifyname
        (:`Slash`
          (`self.SphereTraceDamage` _damageinfo Length Radius))))))

(event `FireBullet`
  (params (TraceStart :type "Vector Structure") (TraceEnd :type "Vector Structure") (DamageInfo :type "/Game/DamageSystem/S_DamageInfo Structure"))
  ;[1 1 1] Attack Notifys
  ;;[0 0 0] Bullet
  (bind (_outhits _returnvalue) (`KismetSystemLibrary.LineTraceMultiForObjects` TraceStart TraceEnd (`|MakeArray` "ObjectTypeQuery3" :!type "EObjectTypeQuery Enum") false (`|MakeArray` (`self.GetOwner`))))
  (if _returnvalue
    (bind _damage_actor (`self.DamageFirstNonTeamMember` _outhits DamageInfo))
    (`AISense_Damage.ReportDamageEvent` _damage_actor (`self.GetOwner`) (`.Amount_2_64864A0D4320D27C3EA14D8019B5EC9D` (break `/Game/DamageSystem/S_DamageInfo` DamageInfo)) (`Actor.K2_GetActorLocation` (`self.GetOwner`)))))

(event `JumpToPlayerAndAttack`
  (params (AttackInfo :type "/Game/Attacks/S_AttackInfo Structure"))
  (bind (_attacktarget _montage _damageinfo) (break `/Game/Attacks/S_AttackInfo` AttackInfo))
  (bind _returnvalue (`self.GetOwner`))
  ;[1 1 1] Melee Attacks
  (bind _mesh (`self.AttackBase` _attacktarget))
  (bind _notifyname (`|PlayMontage` _mesh _montage)
    (:`then`
      (message `/Game/DamageSystem/BPI_Damagable.SetIsInterupable` _returnvalue false))
    (:`OnCompleted`
      (message `/Game/New_AI/AI/BPI_EnemyAI.AttackEnd` _returnvalue _attacktarget :!label _label_5)
      (message `/Game/DamageSystem/BPI_Damagable.SetIsInterupable` _returnvalue true))
    (:`OnInterrupted`
      (goto _label_5))
    (:`OnNotifyBegin`
      (switch `name` _notifyname
        (:`Slash`
          (`self.SphereTraceDamage` _damageinfo 200.0 20.0))
        (:`Jump`
          (`self.JumpToPlayer` _attacktarget))
        (:`AOESlash`
          (`self.AOEDamage` 350.0 _damageinfo))))))

(event `AOEDamage`
  (params (Radius :type "Float (double-precision)") (DamageInfo :type "/Game/DamageSystem/S_DamageInfo Structure") (`Status Effect` :type "/Game/AOE/E_StatusEffect Enum" :default "NewEnumerator0"))
  (bind _returnvalue (`self.GetOwner`))
  ;[1 1 1] Attack Notifys
  ;;[0 0 0] AOEDamage
  (bind _returnvalue_2 (`|SpawnActorFromClass` "/Game/AOE/BP_AOE_Slashing.BP_AOE_Slashing_C" (`KismetMathLibrary.MakeTransform` (`Actor.K2_GetActorLocation` _returnvalue)) "Undefined" "MultiplyWithRoot" null false true false (cast `Pawn` _returnvalue :!pure true)))
  (set `/Game/AOE/BP_AOE_Base.Radius` Radius _returnvalue_2)
  (add `/Game/AOE/BP_AOE_Base.OnAOEOverlapActor` _returnvalue_2 (delegate `SlashAOETick`))
  (`/Game/AOE/BP_AOE_Base.Trigger` _returnvalue_2))

(event `SlashAOETick`
  (params (Actor :type "Actor Object Reference"))
  (bind _returnvalue (`self.GetOwner`))
  ;[1 1 1] Attack Notifys
  ;;[0 0 0] AOEDamage
  (bind _teamnumber (message `/Game/DamageSystem/BPI_Damagable.GetTeamNumber` Actor))
  (bind _teamnumber_2 (message `/Game/DamageSystem/BPI_Damagable.GetTeamNumber` _returnvalue))
  (if (!= _teamnumber _teamnumber_2)
    (message `/Game/DamageSystem/BPI_Damagable.TakeDamage` Actor (stale `AOEDamage` DamageInfo) _returnvalue (stale `AOEDamage` `Status Effect`))))

(event `Spinning Attack`
  (params (`Attack Info` :type "/Game/Attacks/S_AttackInfo Structure") (`Status Effect` :type "/Game/AOE/E_StatusEffect Enum" :default "NewEnumerator0"))
  (bind (_attacktarget _montage _damageinfo) (break `/Game/Attacks/S_AttackInfo` `Attack Info`))
  (bind _returnvalue (`self.GetOwner`))
  ;[1 1 1] Melee Attacks
  (bind _mesh (`self.AttackBase` _attacktarget))
  (bind _notifyname (`|PlayMontage` _mesh _montage)
    (:`then`
      (message `/Game/DamageSystem/BPI_Damagable.SetIsInterupable` _returnvalue false))
    (:`OnCompleted`
      (message `/Game/New_AI/AI/BPI_EnemyAI.AttackEnd` _returnvalue _attacktarget :!label _label_6)
      (message `/Game/DamageSystem/BPI_Damagable.SetIsInterupable` _returnvalue true))
    (:`OnInterrupted`
      (goto _label_6))
    (:`OnNotifyBegin`
      (switch `name` _notifyname
        (:`Slash`
          (`self.SphereTraceDamage` _damageinfo 200.0 20.0))
        (:`AOESlash`
          (`self.AOEDamage` 300.0 _damageinfo `Status Effect`))))))

(event `SphereTraceDamage`
  (params (DamageInfo :type "/Game/DamageSystem/S_DamageInfo Structure") (Length :type "Float (double-precision)") (Radius :type "Float (single-precision)"))
  (bind _returnvalue (`self.GetOwner`))
  (bind _returnvalue_2 (`Actor.K2_GetActorLocation` _returnvalue))
  ;[1 1 1] Attack Notifys
  ;;[0 0 0] Sphere Trace Damage
  (bind (_outhits _returnvalue_3) (`KismetSystemLibrary.SphereTraceMultiForObjects` _returnvalue_2 (+ _returnvalue_2 (* (`Actor.GetActorForwardVector` _returnvalue) Length)) Radius (`|MakeArray` "ObjectTypeQuery3" :!type "EObjectTypeQuery Enum")))
  (if _returnvalue_3
    (bind _actorsdamaged (`self.DamageAllNonteamMembers` _outhits DamageInfo))
    (for _array_element _actorsdamaged
      _)))

(event `JumpToPlayer`
  (params (AttackTarget :type "Actor Object Reference"))
  (bind _ascharacter (cast `Character` (`self.GetOwner`) :!pure true))
  ;[1 1 1] Attack Notifys
  ;;[0 0 0] Jump to Player
  (bind _location (`self.CalculateFutureActorLocation` AttackTarget))
  (bind _outlaunchvelocity (`GameplayStatics.SuggestProjectileVelocity_CustomArc` (`Actor.K2_GetActorLocation` (`self.GetOwner`)) (`KismetMathLibrary.MakeVector` (.x _location) (.y _location) (+ (.z _location) 100.0)) 0.0 (`KismetMathLibrary.Lerp` 0.5 0.94 (`KismetMathLibrary.FClamp` (`KismetMathLibrary.NormalizeToRange` (`Actor.GetDistanceTo` AttackTarget (`self.GetOwner`)) 400.0 800.0)))))
  (`Character.LaunchCharacter` _ascharacter _outlaunchvelocity true true)
  (add `Character.LandedDelegate` _ascharacter (delegate `OnLand`)))

(event `OnLand`
  (params (Hit :type "HitResult Structure (by ref)"))
  (bind _ascharacter (cast `Character` (`self.GetOwner`) :!pure true))
  ;[1 1 1] Attack Notifys
  ;;[0 0 0] Jump to Player
  (remove `Character.LandedDelegate` _ascharacter (delegate `OnLand`))
  (`MovementComponent.StopMovementImmediately` (`Character.CharacterMovement` _ascharacter)))

(event `HealEnd`)

(fn `AttackBase`
  (params (`Attack Target` :type "Actor Object Reference"))
  (returns (Mesh :type "SkeletalMeshComponent Object Reference"))
  (bind _returnvalue (`self.GetOwner`))
  (message `/Game/New_AI/AI/BPI_EnemyAI.Attack` _returnvalue `Attack Target`)
  (return (`Actor.GetComponentByClass` _returnvalue "/Script/Engine.SkeletalMeshComponent")))

(fn `CalculateFutureActorLocation`
  (params (Actor :type "Actor Object Reference") (Time :type "Float (double-precision)" :default 1.0))
  (returns (Location :type "Vector Structure"))
  (return (+ (`Actor.K2_GetActorLocation` Actor) (* (* (`Actor.GetVelocity` Actor) (1.0 1.0 0.0)) Time))))

(fn `DamageAllNonteamMembers`
  (params (Hits :type "Array of HitResult Structure") (DamageInfo :type "/Game/DamageSystem/S_DamageInfo Structure"))
  (returns (ActorsDamaged :type "Array of Actor Object Reference"))
  (locals (ActorsDamagedSoFar :type "Array of Actor Object Reference"))
  (for _array_element Hits
    (bind (_bblockinghit _binitialoverlap _time _distance _location _impactpoint _normal _impactnormal _physmat _hitactor) (`GameplayStatics.BreakHitResult` _array_element))
    (bind _teamnumber (message `/Game/DamageSystem/BPI_Damagable.GetTeamNumber` _hitactor))
    (bind _teamnumber_2 (message `/Game/DamageSystem/BPI_Damagable.GetTeamNumber` (`self.GetOwner`)))
    (if (and (!= _teamnumber _teamnumber_2) (not (`KismetArrayLibrary.Array_Contains` (`local.ActorsDamagedSoFar`) _hitactor)))
      (message `/Game/DamageSystem/BPI_Damagable.TakeDamage` _hitactor DamageInfo (`self.GetOwner`) "NewEnumerator0")
      (`KismetArrayLibrary.Array_AddUnique` (`local.ActorsDamagedSoFar`) _hitactor)))
  (return (`local.ActorsDamagedSoFar`)))

(fn `DamageFirstNonTeamMember`
  (params (Hits :type "Array of HitResult Structure") (DamageInfo :type "/Game/DamageSystem/S_DamageInfo Structure"))
  (returns (`Damage Actor` :type "Actor Object Reference"))
  (for _array_element Hits
    (bind (_bblockinghit _binitialoverlap _time _distance _location _impactpoint _normal _impactnormal _physmat _hitactor) (`GameplayStatics.BreakHitResult` _array_element))
    (bind _teamnumber (message `/Game/DamageSystem/BPI_Damagable.GetTeamNumber` _hitactor))
    (bind _teamnumber_2 (message `/Game/DamageSystem/BPI_Damagable.GetTeamNumber` (`self.GetOwner`)))
    (if (!= _teamnumber _teamnumber_2)
      (message `/Game/DamageSystem/BPI_Damagable.TakeDamage` _hitactor DamageInfo (`self.GetOwner`) "NewEnumerator0")
      (`|ExecutionSequence`
        (:`then_0`
          (break))
        (:`then_1`
          (return _hitactor))))))

(fn `Heal`
  (params (Amount :type "Float (double-precision)"))
  (returns (NewHealth :type "Float (double-precision)"))
  (return 0.0))