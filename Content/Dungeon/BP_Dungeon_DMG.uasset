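; BP_Dungeon_DMG is a dungeon actor that spawns a damage-increase pickup when the hero enters its trigger.
; An overlap on the SpawnHealth component by an actor tagged "Hero" spawns BP_DMG_Inrease_PickUp at the SpecialSpawn component's location and rotation.
; The trigger component then destroys itself, so the reward spawns only once, despite its health-related name.
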(event `self.spawn Health.OnComponentBeginOverlap`
  (params (OverlappedComponent :type "PrimitiveComponent Object Reference") (OtherActor :type "Actor Object Reference") (OtherComp :type "PrimitiveComponent Object Reference") (OtherBodyIndex :type Integer) (bFromSweep :type Boolean) (SweepResult :type "HitResult Structure (by ref)"))
  (bind _special_spawn (`self.special spawn`))
  (if (`self.ActorHasTag` OtherActor "Hero")
    (`|SpawnActorFromClass` "/Game/Dungeon/BP_DMG_Inrease_PickUp.BP_DMG_Inrease_PickUp_C" (`KismetMathLibrary.MakeTransform` (`SceneComponent.K2_GetComponentLocation` _special_spawn) (`SceneComponent.K2_GetComponentRotation` _special_spawn)) "AlwaysSpawn" "MultiplyWithRoot" null null)
    (`ActorComponent.K2_DestroyComponent` (`self.spawn Health`))))

(fn `UserConstructionScript`
  (`parent.UserConstructionScript`))