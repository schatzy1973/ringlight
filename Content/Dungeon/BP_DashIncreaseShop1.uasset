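; Shop pickup, named as a dash upgrade, that sells the third-person character a stat increase for coins.
; Entering its box shows a WBP_HealthInteract widget and, if CoinsCollected covers Cost, buys immediately without any input.
; A purchase deducts the coins, raises the first stat enumerator through BPCStats, plays a charm sound and destroys the actor.
; Leaving the box removes the widget.
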(event `self.Box.OnComponentBeginOverlap`
  (params (OverlappedComponent :type "PrimitiveComponent Object Reference") (OtherActor :type "Actor Object Reference") (OtherComp :type "PrimitiveComponent Object Reference") (OtherBodyIndex :type Integer) (bFromSweep :type Boolean) (SweepResult :type "HitResult Structure (by ref)"))
  (bind _cost (`self.Cost`))
  (bind _asbp_third_person_character (cast `/Game/ThirdPerson/Blueprints/BP_ThirdPersonCharacter` OtherActor))
  (`/Engine/EditorBlueprintResources/StandardMacros.IsValid` _asbp_third_person_character
    (:`Is Valid`
      (bind _returnvalue (`|CreateWidget` "/Game/Dungeon/WBP_HealthInteract.WBP_HealthInteract_C"))
      (bind _output_get (set `self.NewVar_1` _returnvalue))
      (`UserWidget.AddToPlayerScreen` _output_get 0)
      (bind _coins_collected (`/Game/ThirdPerson/Blueprints/BP_ThirdPersonCharacter.Coins Collected` _asbp_third_person_character))
      (if (>= _coins_collected _cost)
        (set `/Game/ThirdPerson/Blueprints/BP_ThirdPersonCharacter.Coins Collected` (- _coins_collected _cost) _asbp_third_person_character)
        (`/Game/Souls/Blueprints/BPC_Stats.Increase value` (`/Game/ThirdPerson/Blueprints/BP_ThirdPersonCharacter.BPC_Stats` _asbp_third_person_character) "NewEnumerator0" 15.0)
        (`GameplayStatics.PlaySound2D` "/Game/Sounds/344696__scrampunk__charm.344696__scrampunk__charm" 1.0 1.0 0.0 null null)
        (`self.K2_DestroyActor`)))))

(event `self.Box.OnComponentEndOverlap`
  (params (OverlappedComponent :type "PrimitiveComponent Object Reference") (OtherActor :type "Actor Object Reference") (OtherComp :type "PrimitiveComponent Object Reference") (OtherBodyIndex :type Integer))
  (bind _asbp_third_person_character (cast `/Game/ThirdPerson/Blueprints/BP_ThirdPersonCharacter` OtherActor))
  (`/Engine/EditorBlueprintResources/StandardMacros.IsValid` _asbp_third_person_character
    (:`Is Valid`
      (`Widget.RemoveFromParent` (`self.NewVar_1`)))))

(fn `UserConstructionScript`)