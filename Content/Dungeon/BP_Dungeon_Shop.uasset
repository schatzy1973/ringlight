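; BP_Dungeon_Shop is a dungeon shop that spawns items and sells a magic stance to the player.
; SpawnShopItems places a random pick from PossibleSpawnItems at each spawn-location child, using the dungeon generator's seeded random stream.
; Overlapping MageStance shows an interact widget and, if coins cover Cost, immediately deducts them and calls MagicStance on the player.
; The widget is removed when a Hero-tagged actor leaves.
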(event `self.ReceiveBeginPlay`
  (`parent.ReceiveBeginPlay`)
  (bind _returnvalue (`|CreateWidget` "/Game/Dungeon/WBP_IceInteract.WBP_IceInteract_C"))
  (set `self.NewVar_0` _returnvalue))

(event `self.Mage Stance.OnComponentBeginOverlap`
  (params (OverlappedComponent :type "PrimitiveComponent Object Reference") (OtherActor :type "Actor Object Reference") (OtherComp :type "PrimitiveComponent Object Reference") (OtherBodyIndex :type Integer) (bFromSweep :type Boolean) (SweepResult :type "HitResult Structure (by ref)"))
  (bind _cost (`self.Cost`))
  (bind _asbp_player (cast `/Game/Player/BP_Player` OtherActor))
  (`/Engine/EditorBlueprintResources/StandardMacros.IsValid` _asbp_player
    (:`Is Valid`
      (`UserWidget.AddToPlayerScreen` (`self.NewVar_0`) 0)
      (bind _coins_collected (`/Game/Player/BP_Player.Coins Collected` _asbp_player))
      (if (>= _coins_collected _cost)
        (set `/Game/Player/BP_Player.Coins Collected` (- _coins_collected _cost) _asbp_player)
        (`/Game/Player/BP_Player.MagicStance` _asbp_player)))))

(event `self.Mage Stance.OnComponentEndOverlap`
  (params (OverlappedComponent :type "PrimitiveComponent Object Reference") (OtherActor :type "Actor Object Reference") (OtherComp :type "PrimitiveComponent Object Reference") (OtherBodyIndex :type Integer))
  (if (`self.ActorHasTag` OtherActor "Hero")
    (`Widget.RemoveFromParent` (`self.NewVar_0`))))

(event `/Game/Dungeon/BPI_SpawnShopItems.SpawnShopItems`
  (`self.SpawnItems`))

(event `SpawnItems`
  (bind _returnvalue (`GameplayStatics.GetActorOfClass` "/Game/Dungeon/BP_Dungeon_Generator.BP_Dungeon_Generator_C"))
  (for _array_element (`SceneComponent.GetChildrenComponents` (`self.ShopItemSpawnLocations`) false)
    (`|SpawnActorFromClass` (`KismetArrayLibrary.Array_RandomFromStream` (`self.PossibleSpawnItems`) (`/Game/Dungeon/BP_Dungeon_Generator.Stream` _returnvalue)) (`KismetMathLibrary.MakeTransform` (`SceneComponent.K2_GetComponentLocation` _array_element)) "Undefined" "MultiplyWithRoot" null null)))

(fn `UserConstructionScript`
  (`parent.UserConstructionScript`))