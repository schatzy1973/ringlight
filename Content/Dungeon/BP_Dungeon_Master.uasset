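; Dungeon actor that deletes itself when none of its priority exits have changed since play began.
; On BeginPlay it records how many arrow components carry the Priority tag.
; CheckShouldDelete recounts them and destroys the actor if the count still matches; nothing in this file removes tags or calls that event.
; An unconnected loop over the ExitsFolder children is left in the graph.
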(event `self.ReceiveBeginPlay`
  (set `self.StartingPriorityExitAmount` (`KismetArrayLibrary.Array_Length` (`self.GetComponentsByTag` "/Script/Engine.ArrowComponent" "Priority"))))

(event `/Game/Dungeon/BPI_DeleteCheck.CheckShouldDelete`
  (if (== (`KismetArrayLibrary.Array_Length` (`self.GetComponentsByTag` "/Script/Engine.ArrowComponent" "Priority")) (`self.StartingPriorityExitAmount`))
    (`self.K2_DestroyActor`)))

(fn `UserConstructionScript`)