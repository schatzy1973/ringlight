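; BP_Dungeon_Boss is a dungeon actor that spawns the boss encounter when the hero enters its trigger.
; When an actor tagged Hero overlaps the SpawnBoss component, it spawns BP_Enemy_Boss at the SpecialSpawn component's location and rotation, ignoring collision.
; It then destroys the SpawnBoss component so the trigger fires only once.
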(event `self.spawn boss.OnComponentBeginOverlap`
  (params (OverlappedComponent :type "PrimitiveComponent Object Reference") (OtherActor :type "Actor Object Reference") (OtherComp :type "PrimitiveComponent Object Reference") (OtherBodyIndex :type Integer) (bFromSweep :type Boolean) (SweepResult :type "HitResult Structure (by ref)"))
  (bind _special_spawn (`self.special spawn`))
  (if (`self.ActorHasTag` OtherActor "Hero")
    (`|SpawnActorFromClass` "/Game/New_AI/Boss_Enemy/BP_Enemy_Boss.BP_Enemy_Boss_C" (`KismetMathLibrary.MakeTransform` (`SceneComponent.K2_GetComponentLocation` _special_spawn) (`SceneComponent.K2_GetComponentRotation` _special_spawn)) "AlwaysSpawn" "MultiplyWithRoot" null 2 null)
    (`ActorComponent.K2_DestroyComponent` (`self.spawn boss`))))

(fn `UserConstructionScript`
  (`parent.UserConstructionScript`))