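; BP_DoorC is a coin-cost dungeon door that is destroyed when a player who can afford it touches it.
; When a BP_Player tagged Hero enters its Box, it creates and shows a WBP_DoorInteract widget.
; If CoinsCollected covers CoinsCost, it deducts the cost and destroys itself immediately, with no input press.
; End overlap by a Hero-tagged actor removes the widget.
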(event `self.ReceiveBeginPlay`
  (cast `/Game/Player/BP_Player` (`GameplayStatics.GetPlayerCharacter` 0))
  (`/Engine/EditorBlueprintResources/StandardMacros.IsValid` null
    (:`Is Valid`
      (bind _returnvalue (`|CreateWidget` "/Game/Dungeon/WBP_DoorInteract.WBP_DoorInteract_C"))
      (set `self.Interact Widget` _returnvalue))))

(event `self.Box.OnComponentBeginOverlap`
  (params (OverlappedComponent :type "PrimitiveComponent Object Reference") (OtherActor :type "Actor Object Reference") (OtherComp :type "PrimitiveComponent Object Reference") (OtherBodyIndex :type Integer) (bFromSweep :type Boolean) (SweepResult :type "HitResult Structure (by ref)"))
  (bind _asbp_player (cast `/Game/Player/BP_Player` OtherActor))
  (bind _output_get (set `self.As BP Player` _asbp_player))
  (if (`self.ActorHasTag` OtherActor "Hero")
    (bind _returnvalue (`|CreateWidget` "/Game/Dungeon/WBP_DoorInteract.WBP_DoorInteract_C"))
    (set `self.Interact Widget` _returnvalue)
    (`UserWidget.AddToPlayerScreen` (`self.Interact Widget`) 0)
    (bind _coins_collected (`/Game/Player/BP_Player.Coins Collected` _output_get))
    (if (>= _coins_collected (`self.Coins Cost`))
      (set `/Game/Player/BP_Player.Coins Collected` (- _coins_collected (`self.Coins Cost`)) _output_get)
      (`self.K2_DestroyActor`))))

(event `self.Box.OnComponentEndOverlap`
  (params (OverlappedComponent :type "PrimitiveComponent Object Reference") (OtherActor :type "Actor Object Reference") (OtherComp :type "PrimitiveComponent Object Reference") (OtherBodyIndex :type Integer))
  (if (`self.ActorHasTag` OtherActor "Hero")
    (`Widget.RemoveFromParent` (`self.Interact Widget`))))

(fn `UserConstructionScript`)